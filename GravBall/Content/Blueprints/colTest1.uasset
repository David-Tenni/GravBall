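; colTest1 is a test actor that moves back and forth, reversing when it begins overlapping a Frame actor.
; Each tick it offsets itself by MovementDirection along world Y with sweep when UpAxis is true, otherwise along Z without sweep.
; On overlap it prints the other actor's name, and a successful cast to Frame calls ChangeDirection, which negates MovementDirection.
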(event `self.ReceiveActorBeginOverlap`
  (params (OtherActor :type "Actor Object Reference"))
  (`KismetSystemLibrary.PrintString` (`KismetSystemLibrary.GetDisplayName` OtherActor))
  (cast `/Game/Blueprints/Frame` OtherActor)
  (`self.ChangeDirection`))

(event `self.ReceiveTick`
  (params (DeltaSeconds :type "Float (single-precision)"))
  (bind _movement_direction (`self.Movement Direction`))
  (if (`self.UpAxis`)
    (`self.K2_AddActorWorldOffset` (`KismetMathLibrary.MakeVector` 0.0 _movement_direction) true)
    (else
      (`self.K2_AddActorWorldOffset` (`KismetMathLibrary.MakeVector` 0.0 0.0 _movement_direction)))))

(fn `ChangeDirection`
  (set `self.Movement Direction` (* (`self.Movement Direction`) -1.0)))

(fn `UserConstructionScript`)